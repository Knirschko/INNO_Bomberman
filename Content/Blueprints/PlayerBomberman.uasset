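; Player character for a 2D Bomberman-style game that moves, plants bombs, collects stat upgrades and opens pause and game-over screens.
; Bombs snap to the GridManager's closest cell, capped by a live count that drops through each bomb's destroy event.
; Upgrade functions raise bomb limit, flame range and fly speed.
; An unfinished Tick-driven animation handler swaps between side and front-idle flipbooks based on velocity.
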(event `InputAction|PlantBomb`
  (params (Key :type "Key Structure"))
  ;[1 1 1] spawn bomb
  (:`Pressed`
    (`/Engine/EditorBlueprintResources/StandardMacros.CompareInt` (`self.MaxBombs`) (`self.CurrentBombs`)
      (:`>`
        (bind _returnvalue (`GameplayStatics.GetActorOfClass` "/Game/Grid/GridManager.GridManager_C"))
        (bind _outputvector (`/Game/Grid/GridManager.Get Closest Grid Position` _returnvalue (`self.K2_GetActorLocation`)))
        (bind _returnvalue_2 (`|SpawnActorFromClass` "/Game/Blueprints/Bomb.Bomb_C" (`KismetMathLibrary.Conv_VectorToTransform` _outputvector) "Undefined" "OverrideRootScale" null null))
        (`/Engine/EditorBlueprintResources/StandardMacros.IncrementInt` (`self.CurrentBombs`)
          (:`  `
            (add `self.OnDestroyed` _returnvalue_2 (delegate `DestoryedBomb`))))))))

(event `InputAction|OpenPauseMenu`
  (params (Key :type "Key Structure"))
  (bind _returnvalue (`GameplayStatics.GetPlayerController` 0))
  (bind _returnvalue_2 (`GameplayStatics.GetPlayerController` 0))
  ;[1 1 1] Basic Movement and Skills
  ;;[1 1 1] Pause
  (:`Pressed`
    (`/Engine/EditorBlueprintResources/StandardMacros.FlipFlop`
      (:`A`
        (bind _returnvalue_3 (`|GenericCreateObject` "/Game/UI/PauseMenu.PauseMenu_C"))
        (`UserWidget.AddToViewport` _returnvalue_3 0)
        (`GameplayStatics.SetGamePaused` true)
        (`WidgetBlueprintLibrary.SetInputMode_GameAndUIEx` _returnvalue_2 null)
        (set `PlayerController.bShowMouseCursor` true _returnvalue_2))
      (:`B`
        (`Widget.RemoveFromParent` _returnvalue_3)
        (`WidgetBlueprintLibrary.SetInputMode_GameOnly` _returnvalue)
        (set `PlayerController.bShowMouseCursor` false _returnvalue)
        (`GameplayStatics.SetGamePaused` false)))))

(event `DestoryedBomb` :!signature `self.OnDestroyed`
  (params (DestroyedActor :type "Actor Object Reference"))
  ;[1 1 1] spawn bomb
  (`/Engine/EditorBlueprintResources/StandardMacros.DecrementInt` (`self.CurrentBombs`)))

(event `InputAxis|MoveRight`
  (params (AxisValue :type "Float (single-precision)"))
  ;[1 1 1] Basic Movement and Skills
  ;;[1 1 1] Movement
  (`self.AddMovementInput` (1.0 0.0 0.0) AxisValue))

(event `self.ReceiveBeginPlay`)

(event `self.ReceiveTick`
  (params (DeltaSeconds :type "Float (single-precision)"))
  (`self.AnimationHandler`))

(event `InputAxis|MoveUp`
  (params (AxisValue :type "Float (single-precision)"))
  ;[1 1 1] Basic Movement and Skills
  ;;[1 1 1] Movement
  (`self.AddMovementInput` (0.0 1.0 0.0) AxisValue))

(event `AnimationHandler`
  ;[1 1 1] Animations NOT FINISHED (#moonwalk)
  (`PaperFlipbookComponent.SetFlipbook` (`self.Sprite`) (select `bool` (> (`KismetMathLibrary.VSize` (`MovementComponent.Velocity` (`self.CharacterMovement`))) 0.0) :`false` "/Game/Sprites/Bomberman/Front/Idle_Front_Bomberman.Idle_Front_Bomberman" :`true` "/Game/Sprites/Bomberman/Side/Side_Bomberman.Side_Bomberman" :!type "PaperFlipbook Object Reference")))

(fn `GameOver`
  (bind _returnvalue (`GameplayStatics.GetPlayerController` 0))
  (bind _returnvalue_2 (`|GenericCreateObject` "/Game/UI/GameOverScreen.GameOverScreen_C"))
  (`UserWidget.AddToViewport` _returnvalue_2 0)
  (`GameplayStatics.SetGamePaused` true)
  (`WidgetBlueprintLibrary.SetInputMode_GameAndUIEx` _returnvalue null)
  (set `PlayerController.bShowMouseCursor` true _returnvalue))

(fn `increaseFlameRange`
  (`/Engine/EditorBlueprintResources/StandardMacros.IncrementInt` (`self.FlameRange`)))

(fn `increaseMaxBombs`
  (`/Engine/EditorBlueprintResources/StandardMacros.IncrementInt` (`self.MaxBombs`)))

(fn `increaseMaxSpeed`
  (bind _charactermovement (`self.CharacterMovement`))
  (set `CharacterMovementComponent.MaxFlySpeed` (+ (`CharacterMovementComponent.MaxFlySpeed` _charactermovement) 30.0) _charactermovement))

(fn `UserConstructionScript`)