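; MindMaker actor that links the game to an external reinforcement learning server over local SocketIO, as a template with placeholder observation and reward logic.
; BeginPlay calls MindMakerWindows, and on socket connection it binds events and sends algorithm and training settings as JSON.
; Each received action is parsed and stored, then DelayForDisplay sends back observations, reward and done state.
; Server messages flag training completion or quit the game after evaluation.
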(event `Delay for display`
  (`self.MakeObservations`)
  (`self.CheckReward`)
  (setmembers `/Game/MindMaker/MindMakerDRLStarterContent/Assets/MindMakerDRLStarterContent/MindMakerCustStrucStart` :`StructRef` (`self.MindMakerStruct`) :`reward` (`self.Reward`) :`observations` (`self.Observations`) :`done` (`self.done`))
  (`SocketIOClientComponent.Emit` (`self.SocketIOClient`) "sendobs" (`SIOJLibrary.Conv_StringToJsonValue` (`SIOJsonObject.EncodeJson` (`SIOJLibrary.StructToJsonObject` (`self.MindMakerStruct`)))) "/"))

(event `self.SocketIOClient.OnConnected`
  (params (SessionId :type String) (bIsReconnection :type Boolean))
  (`SocketIOClientComponent.BindEventToFunction` (`self.SocketIOClient`) "messages" "Messages" null "/" "USE_DEFAULT")
  (`SocketIOClientComponent.BindEventToFunction` (`self.SocketIOClient`) "reaction" "ReceiveAction" null "/" "USE_DEFAULT")
  (`SocketIOClientComponent.BindEventToFunction` (`self.SocketIOClient`) "sendobs" "SendObservations" null "/" "USE_DEFAULT")
  (`SocketIOClientComponent.Connect` (`self.SocketIOClient`) "http://localhost:3000" "socket.io" null null)
  (`self.LaunchMindMaker` "NewEnumerator3" (`self.NumTrainingEpisodes`) (`self.NumEvalEpisodes`) false true false true "" (`KismetStringLibrary.Conv_IntToString` (`self.MaxActions`)) "" false (`self.A2cparams`) (`self.AcerParams`) (`self.AcktrParams`) (`self.DqnParams`) (`self.Ppo2Params`) (`self.SacParams`) (`self.Td3Params`)))

(event `self.ReceiveBeginPlay`
  (`MindMakerBPLibrary.MindMakerWindows`)
  (`KismetSystemLibrary.PrintString` "MindMaker Launched"))

(fn `CheckReward`
  (if true
    _))

(fn `LaunchMindMaker`
  (params (`RL Algorithm` :type "/Game/MindMaker/MindMakerDRLStarterContent/Assets/MindMakerDRLStarterContent/LearningAlgorithmsStart Enum" :default "NewEnumerator3") (NumTrainEp :type Integer) (NumEvalEp :type Integer) (ContinousActionSpace :type Boolean) (DiscreteActionSpace :type Boolean) (LoadPreTrainedModel :type Boolean) (SaveModelAfterTraining :type Boolean) (`Save/LoadModelName` :type String) (ActionSpaceShape :type String) (ObservationSpaceShape :type String) (UseCustomParams :type Boolean) (A2cCustomParams :type "/Game/MindMaker/Examples/Assets/MatchToSample/A2cCustomParameters Structure") (AcerCustomParams :type "/Game/MindMaker/Examples/Assets/MatchToSample/AcerCustomParameters Structure") (AcktrCustomParams :type "/Game/MindMaker/Examples/Assets/MatchToSample/AcktrCustomParameters Structure") (DqnCustomParams :type "/Game/MindMaker/Examples/Assets/MatchToSample/DqnCustomParameters Structure") (Ppo2CustomParams :type "/Game/MindMaker/Examples/Assets/MatchToSample/PPO2CustomParameters Structure") (SacCustomParams :type "/Game/MindMaker/Examples/Assets/MatchToSample/SacCustomParameters Structure") (Td3CustomParams :type "/Game/MindMaker/Examples/Assets/MatchToSample/Td3CustomParameters Structure"))
  (setmembers `/Game/MindMaker/MindMakerDRLStarterContent/Assets/MindMakerDRLStarterContent/MindMakerCustStrucStart` :`StructRef` (`self.ExampleStruct`) :`reward` (`self.Reward`) :`observations` (`self.Observations`) :`trainepisodes` NumTrainEp :`evalepisodes` NumEvalEp :`maxactions` (`self.MaxActions`) :`loadmodel` (`KismetStringLibrary.Conv_BoolToString` LoadPreTrainedModel) :`savemodel` (`KismetStringLibrary.Conv_BoolToString` SaveModelAfterTraining) :`algselected` `RL Algorithm` :`customparams` (`KismetStringLibrary.Conv_BoolToString` UseCustomParams) :`a2cparams` A2cCustomParams :`acerparams` AcerCustomParams :`acktrparams` AcktrCustomParams :`dqnparams` DqnCustomParams :`ddpgparams` (struct :`policy` "NewEnumerator17" :`gamma` 0.99 :`verbose` 1 :`initsetupmodel` "True" :`fulltensorboardlog` "False" :`ncputfsess` "1" :`layers` "[64, 64]" :`buffersize` "50000" :`nbtrainsteps` 50 :`nbrolloutsteps` 100 :`nbevalsteps` 100 :`normalizeobservations` "False" :`tau` 0.001 :`paramnoiseadaptioninterval` 50 :`normalize_returns` "False" :`enable_popart` "False" :`observation_range` "(-5.0, 5.0)" :`critic_l2_reg` "0.0" :`actor_lr` 0.0001 :`critic_lr` 0.001 :`reward_scale` 1.0 :`render` "False" :`render_eval` "False" :`random_exploration` "0.0" :`act_func` "NewEnumerator3") :`ppo1params` (struct :`policy` "NewEnumerator3" :`gamma` 0.99 :`verbose` 1 :`_init_setup_model` "True" :`full_tensorboard_log` "False" :`n_cpu_tf_sess` "1" :`layers` "[64, 64]" :`timesteps_per_actorbatch` 256 :`clip_param` 0.2 :`entcoeff` 0.01 :`optim_epochs` 4.0 :`optim_stepsize` 0.001 :`optim_batchsize` 64 :`lam` 0.95 :`adam_epsilon` 5e-05 :`schedule` "linear" :`act_func` "NewEnumerator3") :`ppo2params` Ppo2CustomParams :`sacparams` SacCustomParams :`td3params` Td3CustomParams :`trpoparams` (struct :`policy` "NewEnumerator3" :`gamma` 0.99 :`verbose` 1 :`_init_setup_model` "True" :`full_tensorboard_log` "False" :`n_cpu_tf_sess` "1" :`layers` "[64, 64]" :`entcoeff` 0.01 :`lam` 0.98 :`timesteps_per_batch` 1024 :`max_kl` 0.01 :`cg_iters` 10 :`cg_damping` 0.01 :`vf_stepsize` 0.0003 :`vf_iters` 3 :`act_func` "NewEnumerator3") :`modelname` `Save/LoadModelName` :`actionspace` ActionSpaceShape :`observationspace` ObservationSpaceShape :`conactionspace` ContinousActionSpace :`disactionspace` DiscreteActionSpace :`done` false)
  (`SocketIOClientComponent.Emit` (`self.SocketIOClient`) "launchmindmaker" (`SIOJLibrary.Conv_StringToJsonValue` (`SIOJsonObject.EncodeJson` (`SIOJLibrary.StructToJsonObject` (`self.MindMakerStruct`)))) "/"))

(fn `MakeObservations`
  (set `self.Observations` (`KismetStringLibrary.Concat_StrStr` "[" "" "]")))

(fn `Messages`
  (params (Message :type "SIOJsonValue Object Reference"))
  (bind _returnvalue (`SIOJsonValue.AsString` Message))
  (`KismetSystemLibrary.PrintString` _returnvalue)
  (if (`KismetStringLibrary.EqualEqual_StrStr` _returnvalue "Training complete")
    (set `self.TrainingComplete` true)
    (elif (`KismetStringLibrary.EqualEqual_StrStr` _returnvalue "Evaluation Complete")
      (`KismetSystemLibrary.PrintString` "Quiting Game")
      (`KismetSystemLibrary.QuitGame` null "Quit"))))

(fn `ReceiveAction`
  (params (Message :type "SIOJsonValue Object Reference"))
  (bind _returnvalue (`KismetStringLibrary.Conv_StringToDouble` (`KismetStringLibrary.Replace` (`KismetStringLibrary.Replace` (`|GetArrayItem` (`KismetStringLibrary.ParseIntoArray` (`SIOJsonValue.AsString` Message))) "[") "]")))
  ;[1 1 1] This recieves results from the neural network and updates the environment
  (set `self.ActionSelected` _returnvalue)
  (set `self.ActionReceived` true)
  (`KismetSystemLibrary.PrintString` (`KismetStringLibrary.Concat_StrStr` "Predicted Action:" (`KismetStringLibrary.Conv_DoubleToString` _returnvalue)))
  (`self.Delay for display`))

(fn `UserConstructionScript`)