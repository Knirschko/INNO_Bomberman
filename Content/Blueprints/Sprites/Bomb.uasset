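; Bomb actor that explodes into flames on a fixed fuse timer started at BeginPlay.
; When the timer fires the boom event, it destroys itself, spawns a Flame at its transform and passes CurrentRange to SpawnFlameRange.
; SetRangeForBomb stores the player's range in CurrentRange.
; A separate DestroyBomb function detonates immediately with a supplied transform and range, though it also sets a timer on its own name.
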(event `boom`
  (`self.K2_DestroyActor`)
  (bind _returnvalue (`|SpawnActorFromClass` "/Game/Blueprints/Sprites/Flame.Flame_C" (`self.GetTransform`) "Undefined" "OverrideRootScale" null null))
  (`/Game/Blueprints/Sprites/Flame.SpawnFlameRange` _returnvalue (`self.currentRange`)))

(event `self.ReceiveBeginPlay`
  (`KismetSystemLibrary.K2_SetTimerDelegate` (delegate `boom`) 3.0))

(fn `DestroyBomb`
  (params (Position :type "Transform Structure") (FireRange :type Integer))
  (`KismetSystemLibrary.K2_SetTimer` null "Destroy Bomb" 3.0)
  (`self.K2_DestroyActor`)
  (bind _returnvalue (`|SpawnActorFromClass` "/Game/Blueprints/Sprites/Flame.Flame_C" Position "Undefined" "OverrideRootScale" null null))
  (`/Game/Blueprints/Sprites/Flame.SpawnFlameRange` _returnvalue FireRange))

(fn `SetRangeForBomb`
  (params (PlayerRange :type Integer))
  (set `self.currentRange` PlayerRange))

(fn `UserConstructionScript`)