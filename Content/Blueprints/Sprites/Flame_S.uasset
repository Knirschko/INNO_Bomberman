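; Short-lived explosion flame for a grid-based, Bomberman-style game that calls GameOver on any overlapping player or enemy.
; Each flame destroys itself on a one-second timer after BeginPlay.
; SpawnFlameRange queries GridManager_S outward in four directions, spawning more Flame_S actors on free tiles up to FlameRange past the adjacent one.
; Occupied tiles halt the spread, and destructible ones are removed and replaced with a flame.
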(event `self.ReceiveActorBeginOverlap`
  (params (OtherActor :type "Actor Object Reference"))
  (bind _asplayer_class_og (cast `/Game/Blueprints/PlayerClass_OG` OtherActor)
    (:`then`
      (`/Game/Blueprints/PlayerClass_OG.GameOver` _asplayer_class_og))
    (:`CastFailed`
      (bind _asenemy_class_og (cast `/Game/Blueprints/AI_enemy/EnemyClass_OG` OtherActor))
      (`/Game/Blueprints/AI_enemy/EnemyClass_OG.GameOver` _asenemy_class_og))))

(event `self.ReceiveBeginPlay`
  ;[1 1 1] burning
  (`KismetSystemLibrary.K2_SetTimerDelegate` (delegate `burn`) 1.0))

(event `burn`
  ;[1 1 1] burning
  (`self.K2_DestroyActor`))

(fn `SpawnFlameRange`
  (params (FlameRange :type Integer))
  (bind _returnvalue (`self.K2_GetActorLocation`))
  (bind _returnvalue_2 (`GameplayStatics.GetActorOfClass` "/Game/Grid/GridManager_S.GridManager_S_C"))
  (`|ExecutionSequence`
    (:`then_0`
      (bind (_occupied _uplocation) (`/Game/Grid/GridManager_S.UpOccupied` _returnvalue_2 _returnvalue))
      (if _occupied
        (bind _destructible (`/Game/Grid/GridManager_S.isDestructible` _returnvalue_2 _uplocation))
        (if _destructible
          (`/Game/Grid/GridManager_S.RemoveExplodableTile` _returnvalue_2 _uplocation)
          (`|SpawnActorFromClass` "Flame_S_C" (`KismetMathLibrary.Conv_VectorToTransform` _uplocation) "Undefined" "OverrideRootScale" null null))
        (else
          (`|SpawnActorFromClass` "Flame_S_C" (`KismetMathLibrary.Conv_VectorToTransform` _uplocation) "Undefined" "OverrideRootScale" null null)
          (set `self.UpLocation` _uplocation)
          (for _ (range 1 (+ FlameRange 1))
            (bind (_occupied_2 _uplocation_2) (`/Game/Grid/GridManager_S.UpOccupied` _returnvalue_2 (`self.UpLocation`)))
            (if _occupied_2
              (bind _destructible_2 (`/Game/Grid/GridManager_S.isDestructible` _returnvalue_2 _uplocation_2))
              (if _destructible_2
                (`/Game/Grid/GridManager_S.RemoveExplodableTile` _returnvalue_2 _uplocation_2)
                (`|SpawnActorFromClass` "Flame_S_C" (`KismetMathLibrary.Conv_VectorToTransform` _uplocation_2) "Undefined" "OverrideRootScale" null null)
                (break))
              (else
                (`|SpawnActorFromClass` "Flame_S_C" (`KismetMathLibrary.Conv_VectorToTransform` _uplocation_2) "Undefined" "OverrideRootScale" null null)
                (set `self.UpLocation` _uplocation_2)))))))
    (:`then_1`
      (bind (_occupied_3 _downlocation) (`/Game/Grid/GridManager_S.DownOccupied` _returnvalue_2 _returnvalue))
      (if _occupied_3
        (bind _destructible_3 (`/Game/Grid/GridManager_S.isDestructible` _returnvalue_2 _downlocation))
        (if _destructible_3
          (`/Game/Grid/GridManager_S.RemoveExplodableTile` _returnvalue_2 _downlocation)
          (`|SpawnActorFromClass` "Flame_S_C" (`KismetMathLibrary.Conv_VectorToTransform` _downlocation) "Undefined" "OverrideRootScale" null null))
        (else
          (`|SpawnActorFromClass` "Flame_S_C" (`KismetMathLibrary.Conv_VectorToTransform` _downlocation) "Undefined" "OverrideRootScale" null null)
          (set `self.DownLocation` _downlocation)
          (for _ (range 1 (+ FlameRange 1))
            (bind (_occupied_4 _downlocation_2) (`/Game/Grid/GridManager_S.DownOccupied` _returnvalue_2 (`self.DownLocation`)))
            (if _occupied_4
              (bind _destructible_4 (`/Game/Grid/GridManager_S.isDestructible` _returnvalue_2 _downlocation_2))
              (if _destructible_4
                (`/Game/Grid/GridManager_S.RemoveExplodableTile` _returnvalue_2 _downlocation_2)
                (`|SpawnActorFromClass` "Flame_S_C" (`KismetMathLibrary.Conv_VectorToTransform` _downlocation_2) "Undefined" "OverrideRootScale" null null)
                (break))
              (else
                (`|SpawnActorFromClass` "Flame_S_C" (`KismetMathLibrary.Conv_VectorToTransform` _downlocation_2) "Undefined" "OverrideRootScale" null null)
                (set `self.DownLocation` _downlocation_2)))))))
    (:`then_2`
      (bind (_occupied_5 _leftlocation) (`/Game/Grid/GridManager_S.LeftOccupied` _returnvalue_2 _returnvalue))
      (if _occupied_5
        (bind _destructible_5 (`/Game/Grid/GridManager_S.isDestructible` _returnvalue_2 _leftlocation))
        (if _destructible_5
          (`/Game/Grid/GridManager_S.RemoveExplodableTile` _returnvalue_2 _leftlocation)
          (`|SpawnActorFromClass` "Flame_S_C" (`KismetMathLibrary.Conv_VectorToTransform` _leftlocation) "Undefined" "OverrideRootScale" null null))
        (else
          (`|SpawnActorFromClass` "Flame_S_C" (`KismetMathLibrary.Conv_VectorToTransform` _leftlocation) "Undefined" "OverrideRootScale" null null)
          (set `self.LeftLocation` _leftlocation)
          (for _ (range 1 (+ FlameRange 1))
            (bind (_occupied_6 _leftlocation_2) (`/Game/Grid/GridManager_S.LeftOccupied` _returnvalue_2 (`self.LeftLocation`)))
            (if _occupied_6
              (bind _destructible_6 (`/Game/Grid/GridManager_S.isDestructible` _returnvalue_2 _leftlocation_2))
              (if _destructible_6
                (`/Game/Grid/GridManager_S.RemoveExplodableTile` _returnvalue_2 _leftlocation_2)
                (`|SpawnActorFromClass` "Flame_S_C" (`KismetMathLibrary.Conv_VectorToTransform` _leftlocation_2) "Undefined" "OverrideRootScale" null null)
                (break))
              (else
                (`|SpawnActorFromClass` "Flame_S_C" (`KismetMathLibrary.Conv_VectorToTransform` _leftlocation_2) "Undefined" "OverrideRootScale" null null)
                (set `self.LeftLocation` _leftlocation_2)))))))
    (:`then_3`
      (bind (_occupied_7 _rightlocation) (`/Game/Grid/GridManager_S.RightOccupied` _returnvalue_2 _returnvalue))
      (if _occupied_7
        (bind _destructible_7 (`/Game/Grid/GridManager_S.isDestructible` _returnvalue_2 _rightlocation))
        (if _destructible_7
          (`/Game/Grid/GridManager_S.RemoveExplodableTile` _returnvalue_2 _rightlocation)
          (`|SpawnActorFromClass` "Flame_S_C" (`KismetMathLibrary.Conv_VectorToTransform` _rightlocation) "Undefined" "OverrideRootScale" null null))
        (else
          (`|SpawnActorFromClass` "Flame_S_C" (`KismetMathLibrary.Conv_VectorToTransform` _rightlocation) "Undefined" "OverrideRootScale" null null)
          (set `self.RightLocation` _rightlocation)
          (for _ (range 1 (+ FlameRange 1))
            (bind (_occupied_8 _rightlocation_2) (`/Game/Grid/GridManager_S.RightOccupied` _returnvalue_2 (`self.RightLocation`)))
            (if _occupied_8
              (bind _destructible_8 (`/Game/Grid/GridManager_S.isDestructible` _returnvalue_2 _rightlocation_2))
              (if _destructible_8
                (`/Game/Grid/GridManager_S.RemoveExplodableTile` _returnvalue_2 _rightlocation_2)
                (`|SpawnActorFromClass` "Flame_S_C" (`KismetMathLibrary.Conv_VectorToTransform` _rightlocation_2) "Undefined" "OverrideRootScale" null null)
                (break))
              (else
                (`|SpawnActorFromClass` "Flame_S_C" (`KismetMathLibrary.Conv_VectorToTransform` _rightlocation_2) "Undefined" "OverrideRootScale" null null)
                (set `self.RightLocation` _rightlocation_2)))))))))

(fn `UserConstructionScript`)