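; Timed bomb actor that explodes into flames a few seconds after it spawns.
; On BeginPlay a one-shot timer fires boom, which destroys the bomb, spawns Flame_OG at its transform and passes it CurrentRange for flame spread.
; SetRangeForBomb stores that range from the supplied player range.
; A separate DestroyBomb function, not called here, explodes immediately at a given position and range, despite also setting a timer by name.
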(event `boom`
  (`self.K2_DestroyActor`)
  (bind _returnvalue (`|SpawnActorFromClass` "/Game/Blueprints/Sprites/Flame_OG.Flame_OG_C" (`self.GetTransform`) "Undefined" "OverrideRootScale" null null))
  (`/Game/Blueprints/Sprites/Flame_OG.SpawnFlameRange` _returnvalue (`self.currentRange`)))

(event `self.ReceiveBeginPlay`
  (`KismetSystemLibrary.K2_SetTimerDelegate` (delegate `boom`) 3.0))

(fn `DestroyBomb`
  (params (Position :type "Transform Structure") (FireRange :type Integer))
  (`KismetSystemLibrary.K2_SetTimer` null "Destroy Bomb" 3.0)
  (`self.K2_DestroyActor`)
  (bind _returnvalue (`|SpawnActorFromClass` "/Game/Blueprints/Sprites/Flame_OG.Flame_OG_C" Position "Undefined" "OverrideRootScale" null null))
  (`/Game/Blueprints/Sprites/Flame_OG.SpawnFlameRange` _returnvalue FireRange))

(fn `SetRangeForBomb`
  (params (PlayerRange :type Integer))
  (set `self.currentRange` PlayerRange))

(fn `UserConstructionScript`)