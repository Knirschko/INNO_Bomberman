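; Max speed pickup item that boosts a player's maximum speed when they overlap it.
; On overlap it casts the other actor to PlayerClass and calls IncreaseMaxSpeed on it.
; It then prints every player's MaxFlySpeed as debug output and passes its own location to the GridManager's ItemRemove, leaving removal to that manager.
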(event `self.ReceiveActorBeginOverlap`
  (params (OtherActor :type "Actor Object Reference"))
  (bind _asplayer_class (cast `/Game/Blueprints/PlayerClass` OtherActor))
  (`/Game/Blueprints/PlayerClass.increaseMaxSpeed` _asplayer_class)
  (bind _outactors (`GameplayStatics.GetAllActorsOfClass` "/Game/Blueprints/PlayerClass.PlayerClass_C"))
  (for _array_element _outactors
    (`KismetSystemLibrary.PrintString` (`KismetStringLibrary.Conv_DoubleToString` (`CharacterMovementComponent.MaxFlySpeed` (`Character.CharacterMovement` _array_element)))))
  (bind _returnvalue (`GameplayStatics.GetActorOfClass` "/Game/Grid/GridManager.GridManager_C"))
  (`/Game/Grid/GridManager.ItemRemove` _returnvalue (`self.K2_GetActorLocation`)))

(fn `UserConstructionScript`)