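; AI_Character_BP is a sprite-based character Blueprint that, despite its AI name, moves from second-player input axes.
; The MoveRight/LeftPL2 and MoveUp/DownPL2 axis events pass their values to MoveLeftRight and MoveUpDown.
; Those functions add movement input along the sprite's world-space forward and up vectors, so motion follows the sprite's orientation.
; It contains no AI logic, and the construction script is empty.
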(event `InputAxis|MoveRight/LeftPL2`
  (params (AxisValue :type "Float (single-precision)"))
  (`self.moveLeftRight` null AxisValue))

(event `InputAxis|MoveUp/DownPL2`
  (params (AxisValue :type "Float (single-precision)"))
  (`self.moveUpDown` null AxisValue))

(fn `moveLeftRight`
  (params (self2 :type "Pawn Object Reference") (ScaleValue :type "Float (single-precision)"))
  (`self.AddMovementInput` self2 (`KismetMathLibrary.GetForwardVector` (`SceneComponent.K2_GetComponentRotation` (`self.Sprite`))) ScaleValue false))

(fn `moveUpDown`
  (params (self2 :type "Pawn Object Reference") (ScaleValue :type "Float (single-precision)"))
  (`self.AddMovementInput` self2 (`KismetMathLibrary.GetUpVector` (`SceneComponent.K2_GetComponentRotation` (`self.Sprite`))) ScaleValue false))

(fn `UserConstructionScript`)