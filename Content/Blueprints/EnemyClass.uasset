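; EnemyClass is a Bomberman-style flipbook character handling local two-player movement, bomb planting, power-ups, pause and game-over screens.
; The PlayerIndex 0 instance takes both players' input, finding the second via "Player2" tag and casting to PlayerClass for movement, EnemyClass for bombs.
; Bombs snap to GridManager cells, counted against per-player limits until destroyed.
; Power-up functions raise speed, bomb limit and flame range; walk/idle animation is marked unfinished.
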(event `InputAction|PlantBomb`
  (params (Key :type "Key Structure"))
  ;[1 1 1] spawn bomb
  (:`Pressed`
    (if (== (`self.PlayerIndex`) 0)
      (`/Engine/EditorBlueprintResources/StandardMacros.CompareInt` (`self.MaxBombs`) (`self.CurrentBombs`)
        (:`>`
          (bind _returnvalue (`GameplayStatics.GetActorOfClass` "/Game/Grid/GridManager.GridManager_C"))
          (bind _outputvector (`/Game/Grid/GridManager.Get Closest Grid Position` _returnvalue (`self.K2_GetActorLocation`)))
          (bind _returnvalue_2 (`|SpawnActorFromClass` "/Game/Blueprints/Bomb.Bomb_C" (`KismetMathLibrary.Conv_VectorToTransform` _outputvector) "Undefined" "OverrideRootScale" null null))
          (`/Game/Blueprints/Bomb.SetRangeForBomb` _returnvalue_2 (`self.FlameRange`))
          (`/Engine/EditorBlueprintResources/StandardMacros.IncrementInt` (`self.CurrentBombs`)
            (:`  `
              (add `self.OnDestroyed` _returnvalue_2 (delegate `DestoryedBomb`)))))))))

(event `DestoryedBomb` :!signature `self.OnDestroyed`
  (params (DestroyedActor :type "Actor Object Reference"))
  ;[1 1 1] spawn bomb
  (`/Engine/EditorBlueprintResources/StandardMacros.DecrementInt` (`self.CurrentBombs`)))

(event `MoveUp/Down`
  (params (Player :type "Pawn Object Reference") (ScaleValue :type "Float (single-precision)"))
  (`self.AddMovementInput` Player (`KismetMathLibrary.GetUpVector` (`SceneComponent.K2_GetComponentRotation` (`self.Sprite`))) ScaleValue false))

(event `InputAction|PlantBomb_2`
  (params (Key :type "Key Structure"))
  (:`Pressed`
    (if (== (`self.PlayerIndex`) 0)
      (bind _outactors (`GameplayStatics.GetAllActorsWithTag` "Player2"))
      (bind _asenemy_class (cast `/Game/Blueprints/EnemyClass` (`|GetArrayItem` _outactors)))
      (bind _currentbombs2 (`/Game/Blueprints/EnemyClass.CurrentBombs2` _asenemy_class))
      (`/Engine/EditorBlueprintResources/StandardMacros.CompareInt` (`/Game/Blueprints/EnemyClass.MaxBombs2` _asenemy_class) _currentbombs2
        (:`>`
          (bind _returnvalue (`GameplayStatics.GetActorOfClass` "/Game/Grid/GridManager.GridManager_C"))
          (bind _outputvector (`/Game/Grid/GridManager.Get Closest Grid Position` _returnvalue (`self.K2_GetActorLocation` _asenemy_class)))
          (bind _returnvalue_2 (`|SpawnActorFromClass` "/Game/Blueprints/Bomb.Bomb_C" (`KismetMathLibrary.Conv_VectorToTransform` _outputvector) "Undefined" "OverrideRootScale" null null))
          (`/Game/Blueprints/Bomb.SetRangeForBomb` _returnvalue_2 (`/Game/Blueprints/EnemyClass.FlameRange2` _asenemy_class))
          (`/Engine/EditorBlueprintResources/StandardMacros.IncrementInt` _currentbombs2
            (:`  `
              (add `self.OnDestroyed` _returnvalue_2 (delegate `CustomEvent`)))))))))

(event `MoveLeft/Right`
  (params (Player :type "Pawn Object Reference") (ScaleValue :type "Float (single-precision)"))
  (`self.AddMovementInput` Player (`KismetMathLibrary.GetForwardVector` (`SceneComponent.K2_GetComponentRotation` (`self.Sprite`))) ScaleValue false))

(event `CustomEvent` :!signature `self.OnDestroyed`
  (params (DestroyedActor :type "Actor Object Reference"))
  (`/Engine/EditorBlueprintResources/StandardMacros.DecrementInt` (`/Game/Blueprints/EnemyClass.CurrentBombs2` (stale `InputAction|PlantBomb_2` _asenemy_class))))

(event `InputAxis|MoveRight/LeftPL2`
  (params (AxisValue :type "Float (single-precision)"))
  (if (== (`self.PlayerIndex`) 0)
    (bind _outactors (`GameplayStatics.GetAllActorsWithTag` "Player2"))
    (bind _asplayer_class (cast `/Game/Blueprints/PlayerClass` (`|GetArrayItem` _outactors)))
    (`self.MoveLeft/Right` (`Controller.K2_GetPawn` (`self.GetController` _asplayer_class)) AxisValue)))

(event `InputAxis|MoveUp/DownPL2`
  (params (AxisValue :type "Float (single-precision)"))
  (if (== (`self.PlayerIndex`) 0)
    (bind _outactors (`GameplayStatics.GetAllActorsWithTag` "Player2"))
    (bind _asplayer_class (cast `/Game/Blueprints/PlayerClass` (`|GetArrayItem` _outactors)))
    (`self.MoveUp/Down` (`Controller.K2_GetPawn` (`self.GetController` _asplayer_class)) AxisValue)))

(event `InputAxis|MoveRight/LeftPL1`
  (params (AxisValue :type "Float (single-precision)"))
  (if (== (`self.PlayerIndex`) 0)
    (`self.MoveLeft/Right` (`Controller.K2_GetPawn` (`self.GetController`)) AxisValue)))

(event `InputAxis|MoveUp/DownPL1`
  (params (AxisValue :type "Float (single-precision)"))
  (if (== (`self.PlayerIndex`) 0)
    (`self.MoveUp/Down` (`Controller.K2_GetPawn` (`self.GetController`)) AxisValue)))

(event `InputAction|OpenPauseMenu`
  (params (Key :type "Key Structure"))
  (bind _returnvalue (`GameplayStatics.GetPlayerController` 0))
  (bind _returnvalue_2 (`GameplayStatics.GetPlayerController` 0))
  ;[1 1 1] Basic Movement and Skills
  ;;[1 1 1] Pause
  (:`Pressed`
    (`/Engine/EditorBlueprintResources/StandardMacros.FlipFlop`
      (:`A`
        (bind _returnvalue_3 (`|GenericCreateObject` "/Game/UI/PauseMenu.PauseMenu_C"))
        (`UserWidget.AddToViewport` _returnvalue_3 0)
        (`GameplayStatics.SetGamePaused` true)
        (`WidgetBlueprintLibrary.SetInputMode_GameAndUIEx` _returnvalue_2 null)
        (set `PlayerController.bShowMouseCursor` true _returnvalue_2))
      (:`B`
        (`Widget.RemoveFromParent` _returnvalue_3)
        (`WidgetBlueprintLibrary.SetInputMode_GameOnly` _returnvalue)
        (set `PlayerController.bShowMouseCursor` false _returnvalue)
        (`GameplayStatics.SetGamePaused` false)))))

(event `self.ReceiveBeginPlay`)

(event `self.ReceiveTick`
  (params (DeltaSeconds :type "Float (single-precision)"))
  (`self.AnimationHandler`))

(event `AnimationHandler`
  ;[1 1 1] Animations NOT FINISHED (#moonwalk)
  (`PaperFlipbookComponent.SetFlipbook` (`self.Sprite`) (select `bool` (> (`KismetMathLibrary.VSize` (`MovementComponent.Velocity` (`self.CharacterMovement`))) 0.0) :`false` "/Game/Sprites/Bomberman/Front/Idle_Front_Bomberman.Idle_Front_Bomberman" :`true` "/Game/Sprites/Bomberman/Side/Side_Bomberman.Side_Bomberman" :!type "PaperFlipbook Object Reference")))

(fn `Down`
  (set `self.Movement` (0.0 -100.0 0.0)))

(fn `GameOver`
  (bind _returnvalue (`GameplayStatics.GetPlayerController` 0))
  (if (`self.ActorHasTag` "Player2")
    (bind _returnvalue_2 (`|GenericCreateObject` "/Game/UI/GameOverScreen_2.GameOverScreen_2_C"))
    (else
      (bind _returnvalue_3 (`|GenericCreateObject` "/Game/UI/GameOverScreen.GameOverScreen_C"))))
  (`UserWidget.AddToViewport` _returnvalue_3 0)
  (`UserWidget.AddToViewport` _returnvalue_2 0)
  (`GameplayStatics.SetGamePaused` true)
  (`WidgetBlueprintLibrary.SetInputMode_GameAndUIEx` _returnvalue null)
  (set `PlayerController.bShowMouseCursor` true _returnvalue))

(fn `increaseFlameRange`
  (if (`self.ActorHasTag` "Player2")
    (bind _result (`/Engine/EditorBlueprintResources/StandardMacros.IncrementInt` (`self.FlameRange2`))
      (:`  `
        (set `self.FlameRange2` _result)))
    (else
      (bind _result_2 (`/Engine/EditorBlueprintResources/StandardMacros.IncrementInt` (`self.FlameRange`))
        (:`  `
          (set `self.FlameRange` _result_2))))))

(fn `increaseMaxBombs`
  (if (`self.ActorHasTag` "Player2")
    (bind _result (`/Engine/EditorBlueprintResources/StandardMacros.IncrementInt` (`self.MaxBombs2`))
      (:`  `
        (set `self.MaxBombs2` _result)))
    (else
      (bind _result_2 (`/Engine/EditorBlueprintResources/StandardMacros.IncrementInt` (`self.MaxBombs`))
        (:`  `
          (set `self.MaxBombs` _result_2))))))

(fn `increaseMaxSpeed`
  (bind _charactermovement (`self.CharacterMovement`))
  (set `CharacterMovementComponent.MaxFlySpeed` (+ (`CharacterMovementComponent.MaxFlySpeed` _charactermovement) 30.0) _charactermovement))

(fn `Left`
  (set `self.Movement` (-100.0 0.0 0.0)))

(fn `Right`
  (set `self.Movement` (100.0 0.0 0.0)))

(fn `Up`
  (set `self.Movement` (0.0 100.0 0.0)))

(fn `UserConstructionScript`)