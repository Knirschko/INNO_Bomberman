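; RandomPlayerClass is a Bomberman sprite character that wanders at random, with empty input axis events.
; Each Tick, a random looping MultiGate picks one of four directions and feeds movement input to the controlled pawn along the sprite's forward or up vector.
; The velocity-based flipbook switch is marked unfinished and its call is disconnected, as is the GameOver screen logic.
; Up, Down, Left and Right only set a Movement vector.
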(event `MoveUp/Down`
  (params (Player :type "Pawn Object Reference") (ScaleValue :type "Float (single-precision)"))
  (`self.moveUpDown` Player ScaleValue))

(event `MoveLeft/Right`
  (params (Player :type "Pawn Object Reference") (ScaleValue :type "Float (single-precision)"))
  (`self.moveLeftRight` Player ScaleValue))

(event `InputAxis|MoveRight/LeftPL1`
  (params (AxisValue :type "Float (single-precision)")))

(event `InputAxis|MoveUp/DownPL1`
  (params (AxisValue :type "Float (single-precision)")))

(event `self.ReceiveBeginPlay`)

(event `self.ReceiveTick`
  (params (DeltaSeconds :type "Float (single-precision)"))
  (bind _returnvalue (`Controller.K2_GetPawn` (`self.GetController`)))
  (`|MultiGate` true true
    (:`Out 0`
      (`self.MoveLeft/Right` _returnvalue 1.0))
    (:`Out 1`
      (`self.MoveLeft/Right` _returnvalue -1.0))
    (:`Out 2`
      (`self.MoveUp/Down` _returnvalue 1.0))
    (:`Out 3`
      (`self.MoveUp/Down` _returnvalue -1.0))))

(event `AnimationHandler`
  ;[1 1 1] Animations NOT FINISHED (#moonwalk)
  (`PaperFlipbookComponent.SetFlipbook` (`self.Sprite`) (select `bool` (> (`KismetMathLibrary.VSize` (`MovementComponent.Velocity` (`self.CharacterMovement`))) 0.0) :`false` "/Game/Sprites/Bomberman/Front/Idle_Front_Bomberman.Idle_Front_Bomberman" :`true` "/Game/Sprites/Bomberman/Side/Side_Bomberman.Side_Bomberman" :!type "PaperFlipbook Object Reference")))

(fn `Down`
  (set `self.Movement` (0.0 -100.0 0.0)))

(fn `GameOver`)

(fn `Left`
  (set `self.Movement` (-100.0 0.0 0.0)))

(fn `moveLeftRight`
  (params (self2 :type "Pawn Object Reference") (ScaleValue :type "Float (single-precision)"))
  (`self.AddMovementInput` self2 (`KismetMathLibrary.GetForwardVector` (`SceneComponent.K2_GetComponentRotation` (`self.Sprite`))) ScaleValue false))

(fn `moveUpDown`
  (params (self2 :type "Pawn Object Reference") (ScaleValue :type "Float (single-precision)"))
  (`self.AddMovementInput` self2 (`KismetMathLibrary.GetUpVector` (`SceneComponent.K2_GetComponentRotation` (`self.Sprite`))) ScaleValue false))

(fn `Right`
  (set `self.Movement` (100.0 0.0 0.0)))

(fn `Up`
  (set `self.Movement` (0.0 100.0 0.0)))

(fn `UserConstructionScript`
  (`parent.UserConstructionScript`))