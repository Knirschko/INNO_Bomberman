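; DangerZone is a short-lived grid hazard actor that marks a cross-shaped flame area and destroys itself on a timer after BeginPlay.
; SpawnDangerZones queries GridManager for neighboring cells in four directions, spawning copies of DangerZone outward until a cell is occupied.
; Each arm reaches up to FlameRange cells beyond the first neighbor.
; Nothing in this file calls that function, and overlap has no logic.
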(event `self.ReceiveActorBeginOverlap`
  (params (OtherActor :type "Actor Object Reference")))

(event `self.ReceiveBeginPlay`
  ;[1 1 1] burning
  (`KismetSystemLibrary.K2_SetTimerDelegate` (delegate `burn`) 3.0))

(event `burn`
  ;[1 1 1] burning
  (`self.K2_DestroyActor`))

(fn `SpawnDangerZones`
  (params (FlameRange :type Integer))
  (bind _returnvalue (`self.K2_GetActorLocation`))
  (bind _returnvalue_2 (`GameplayStatics.GetActorOfClass` "/Game/Grid/GridManager.GridManager_C"))
  (`|ExecutionSequence`
    (:`then_0`
      (bind (_occupied _uplocation) (`/Game/Grid/GridManager.UpOccupied` _returnvalue_2 _returnvalue))
      (if (not _occupied)
        (`|SpawnActorFromClass` "DangerZone_C" (`KismetMathLibrary.Conv_VectorToTransform` _uplocation) "Undefined" "OverrideRootScale" null null)
        (set `self.UpLocation` _uplocation)
        (for _ (range 1 (+ FlameRange 1))
          (bind (_occupied_2 _uplocation_2) (`/Game/Grid/GridManager.UpOccupied` _returnvalue_2 (`self.UpLocation`)))
          (if _occupied_2
            (break)
            (else
              (`|SpawnActorFromClass` "DangerZone_C" (`KismetMathLibrary.Conv_VectorToTransform` _uplocation_2) "Undefined" "OverrideRootScale" null null)
              (set `self.UpLocation` _uplocation_2))))))
    (:`then_1`
      (bind (_occupied_3 _downlocation) (`/Game/Grid/GridManager.DownOccupied` _returnvalue_2 _returnvalue))
      (if (not _occupied_3)
        (`|SpawnActorFromClass` "DangerZone_C" (`KismetMathLibrary.Conv_VectorToTransform` _downlocation) "Undefined" "OverrideRootScale" null null)
        (set `self.DownLocation` _downlocation)
        (for _ (range 1 (+ FlameRange 1))
          (bind (_occupied_4 _downlocation_2) (`/Game/Grid/GridManager.DownOccupied` _returnvalue_2 (`self.DownLocation`)))
          (if _occupied_4
            (break)
            (else
              (`|SpawnActorFromClass` "DangerZone_C" (`KismetMathLibrary.Conv_VectorToTransform` _downlocation_2) "Undefined" "OverrideRootScale" null null)
              (set `self.DownLocation` _downlocation_2))))))
    (:`then_2`
      (bind (_occupied_5 _leftlocation) (`/Game/Grid/GridManager.LeftOccupied` _returnvalue_2 _returnvalue))
      (if (not _occupied_5)
        (`|SpawnActorFromClass` "DangerZone_C" (`KismetMathLibrary.Conv_VectorToTransform` _leftlocation) "Undefined" "OverrideRootScale" null null)
        (set `self.LeftLocation` _leftlocation)
        (for _ (range 1 (+ FlameRange 1))
          (bind (_occupied_6 _leftlocation_2) (`/Game/Grid/GridManager.LeftOccupied` _returnvalue_2 (`self.LeftLocation`)))
          (if _occupied_6
            (break)
            (else
              (`|SpawnActorFromClass` "DangerZone_C" (`KismetMathLibrary.Conv_VectorToTransform` _leftlocation_2) "Undefined" "OverrideRootScale" null null)
              (set `self.LeftLocation` _leftlocation_2))))))
    (:`then_3`
      (bind (_occupied_7 _rightlocation) (`/Game/Grid/GridManager.RightOccupied` _returnvalue_2 _returnvalue))
      (if (not _occupied_7)
        (`|SpawnActorFromClass` "DangerZone_C" (`KismetMathLibrary.Conv_VectorToTransform` _rightlocation) "Undefined" "OverrideRootScale" null null)
        (set `self.RightLocation` _rightlocation)
        (for _ (range 1 (+ FlameRange 1))
          (bind (_occupied_8 _rightlocation_2) (`/Game/Grid/GridManager.RightOccupied` _returnvalue_2 (`self.RightLocation`)))
          (if _occupied_8
            (break)
            (else
              (`|SpawnActorFromClass` "DangerZone_C" (`KismetMathLibrary.Conv_VectorToTransform` _rightlocation_2) "Undefined" "OverrideRootScale" null null)
              (set `self.RightLocation` _rightlocation_2))))))))

(fn `UserConstructionScript`)