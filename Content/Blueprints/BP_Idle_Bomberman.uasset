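; Player-controlled Paper2D Bomberman character with axis movement, grid-snapped bomb planting and a pause menu toggle.
; Bombs spawn at the GridManager's closest position while under MaxBombs; their destroy events free up slots.
; Overlaps check only the first actor of each item class, raising bomb limit, fly speed or flame range.
; Tick swaps idle and side flipbooks by velocity, an animation setup marked unfinished.
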(event `InputAction|PlantBomb`
  (params (Key :type "Key Structure"))
  ;[1 1 1] spawn bomb
  (:`Pressed`
    (`/Engine/EditorBlueprintResources/StandardMacros.CompareInt` (`self.MaxBombs`) (`self.CurrentBombs`)
      (:`>`
        (bind _returnvalue (`GameplayStatics.GetActorOfClass` "/Game/Grid/GridManager.GridManager_C"))
        (bind _outputvector (`/Game/Grid/GridManager.Get Closest Grid Position` _returnvalue (`self.K2_GetActorLocation`)))
        (bind _returnvalue_2 (`|SpawnActorFromClass` "/Game/Blueprints/Bomb.Bomb_C" (`KismetMathLibrary.Conv_VectorToTransform` _outputvector) "Undefined" "OverrideRootScale" null null))
        (`/Engine/EditorBlueprintResources/StandardMacros.IncrementInt` (`self.CurrentBombs`)
          (:`  `
            (add `self.OnDestroyed` _returnvalue_2 (delegate `DestoryedBomb`))))))))

(event `InputAction|PressP` :paused true
  (params (Key :type "Key Structure"))
  (bind _returnvalue (`GameplayStatics.GetPlayerController` 0))
  (bind _returnvalue_2 (`GameplayStatics.GetPlayerController` 0))
  ;[1 1 1] Basic Movement and Skills
  ;;[1 1 1] Pause
  (:`Pressed`
    (`/Engine/EditorBlueprintResources/StandardMacros.FlipFlop`
      (:`A`
        (bind _returnvalue_3 (`|GenericCreateObject` "/Game/UI/PauseMenu.PauseMenu_C"))
        (`UserWidget.AddToViewport` _returnvalue_3 0)
        (`GameplayStatics.SetGamePaused` true)
        (`WidgetBlueprintLibrary.SetInputMode_GameAndUIEx` _returnvalue_2 null)
        (set `PlayerController.bShowMouseCursor` true _returnvalue_2))
      (:`B`
        (`Widget.RemoveFromParent` _returnvalue_3)
        (`WidgetBlueprintLibrary.SetInputMode_GameOnly` _returnvalue)
        (set `PlayerController.bShowMouseCursor` false _returnvalue)
        (`GameplayStatics.SetGamePaused` false)))))

(event `DestoryedBomb` :!signature `self.OnDestroyed`
  (params (DestroyedActor :type "Actor Object Reference"))
  ;[1 1 1] spawn bomb
  (`/Engine/EditorBlueprintResources/StandardMacros.DecrementInt` (`self.CurrentBombs`)))

(event `InputAxis|MoveRight`
  (params (AxisValue :type "Float (single-precision)"))
  ;[1 1 1] Basic Movement and Skills
  ;;[1 1 1] Movement
  (`self.AddMovementInput` (1.0 0.0 0.0) AxisValue))

(event `self.ReceiveBeginPlay`)

(event `self.ReceiveTick`
  (params (DeltaSeconds :type "Float (single-precision)"))
  (`self.AnimationHandler`))

(event `InputAxis|MoveUp`
  (params (AxisValue :type "Float (single-precision)"))
  ;[1 1 1] Basic Movement and Skills
  ;;[1 1 1] Movement
  (`self.AddMovementInput` (0.0 1.0 0.0) AxisValue))

(event `AnimationHandler`
  ;[1 1 1] Animations NOT FINISHED (#moonwalk)
  (`PaperFlipbookComponent.SetFlipbook` (`self.Sprite`) (select `bool` (> (`KismetMathLibrary.VSize` (`MovementComponent.Velocity` (`self.CharacterMovement`))) 0.0) :`false` "/Game/Sprites/Bomberman/Front/Idle_Front_Bomberman.Idle_Front_Bomberman" :`true` "/Game/Sprites/Bomberman/Side/Side_Bomberman.Side_Bomberman" :!type "PaperFlipbook Object Reference")))

(event `self.ReceiveActorBeginOverlap`
  (params (OtherActor :type "Actor Object Reference"))
  (bind _charactermovement (`self.CharacterMovement`))
  (bind _flamerange (`self.FlameRange`))
  ;[1 1 1] all Items
  (`|ExecutionSequence`
    (:`then_0`
      ;;[1 1 1] maxBomb
      (bind _returnvalue (`GameplayStatics.GetActorOfClass` "/Game/Blueprints/Item_MaxBombs.Item_MaxBombs_C"))
      (if (`PrimitiveComponent.IsOverlappingActor` (`self.CapsuleComponent`) _returnvalue)
        (`/Engine/EditorBlueprintResources/StandardMacros.IncrementInt` (`self.MaxBombs`)
          (:`  `
            (`/Game/Blueprints/Item_Class.despawn item` _returnvalue)))))
    (:`then_1`
      ;;[1 1 1] maxSpeed
      (bind _returnvalue_2 (`GameplayStatics.GetActorOfClass` "/Game/Blueprints/Item_MaxSpeed.Item_MaxSpeed_C"))
      (if (`PrimitiveComponent.IsOverlappingActor` (`self.CapsuleComponent`) _returnvalue_2)
        (set `CharacterMovementComponent.MaxFlySpeed` (+ (`CharacterMovementComponent.MaxFlySpeed` _charactermovement) 30.0) _charactermovement)
        (`/Game/Blueprints/Item_Class.despawn item` _returnvalue_2)))
    (:`then_2`
      ;;[1 1 1] maxFlameRange
      (bind _returnvalue_3 (`GameplayStatics.GetActorOfClass` "/Game/Blueprints/Item_FlameRange.Item_FlameRange_C"))
      (if (`PrimitiveComponent.IsOverlappingActor` (`self.CapsuleComponent`) _returnvalue_3)
        (`/Engine/EditorBlueprintResources/StandardMacros.IncrementInt` _flamerange
          (:`  `
            (`/Game/Blueprints/Item_Class.despawn item` _returnvalue_3)
            (`KismetSystemLibrary.PrintText` (`KismetTextLibrary.Conv_IntToText` _flamerange))))))))

(fn `UserConstructionScript`)