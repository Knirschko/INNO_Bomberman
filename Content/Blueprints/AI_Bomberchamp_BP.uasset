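; AI-controlled Bomberchamp pawn Blueprint that moves around the level in fixed grid-sized steps.
; Four directional events each call AIMoveTo on the pawn, targeting a point one fixed step from its current location along X for right and left or Y for up and down.
; MoveUp, MoveDown, MoveLeft and MoveRight functions simply trigger the matching events, exposing the latent moves as callable functions.
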(event `AImoveUp`
  (`|AIMoveTo` self (`KismetMathLibrary.MakeVector` (.x (`self.K2_GetActorLocation`)) (+ (.y (`self.K2_GetActorLocation`)) 64.0) (.z (`self.K2_GetActorLocation`))) null))

(event `AImoveDown`
  (`|AIMoveTo` self (`KismetMathLibrary.MakeVector` (.x (`self.K2_GetActorLocation`)) (+ (.y (`self.K2_GetActorLocation`)) -64.0) (.z (`self.K2_GetActorLocation`))) null))

(event `AImoveRight`
  (`|AIMoveTo` self (`KismetMathLibrary.MakeVector` (+ (.x (`self.K2_GetActorLocation`)) 64.0) (.y (`self.K2_GetActorLocation`)) (.z (`self.K2_GetActorLocation`))) null))

(event `AImoveLeft`
  (`|AIMoveTo` self (`KismetMathLibrary.MakeVector` (+ (.x (`self.K2_GetActorLocation`)) -64.0) (.y (`self.K2_GetActorLocation`)) (.z (`self.K2_GetActorLocation`))) null))

(fn `moveDown`
  (`self.AImoveDown`))

(fn `moveLeft`
  (`self.AImoveLeft`))

(fn `moveRight`
  (`self.AImoveRight`))

(fn `moveUp`
  (`self.AImoveUp`))

(fn `UserConstructionScript`)